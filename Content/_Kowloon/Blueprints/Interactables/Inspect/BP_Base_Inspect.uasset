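; BP_Base_Inspect is a base Blueprint for inspectable interactables that switches the player's view to an inspection camera and back.
; ChangetoInspectionCamera checks that CharacterReference has a valid controller, then uses a FlipFlop to alternate the view target between this actor and the character.
; Each switch starts a camera fade from opaque, masking the cut between views.
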(event `self.ChangeToInspectionCamera`
  (`/Engine/EditorBlueprintResources/StandardMacros.IsValid` (`Pawn.GetController` (`self.CharacterReference`))
    (:`Is Valid`
      (`/Engine/EditorBlueprintResources/StandardMacros.FlipFlop`
        (:`A`
          (`PlayerCameraManager.StartCameraFade` :`self` (`GameplayStatics.GetPlayerCameraManager` 0) :`FromAlpha` 1.0 :`Duration` 3.0)
          (`PlayerController.SetViewTargetWithBlend` (`GameplayStatics.GetPlayerController` 0) self 0.0 "VTBlend_Linear" 0.0 true))
        (:`B`
          (`PlayerCameraManager.StartCameraFade` :`self` (`GameplayStatics.GetPlayerCameraManager` 0) :`FromAlpha` 1.0 :`Duration` 3.0)
          (`PlayerController.SetViewTargetWithBlend` (`GameplayStatics.GetPlayerController` 0) (`self.CharacterReference`) 0.0 "VTBlend_Linear" 0.0 false))))))

(fn `UserConstructionScript`)