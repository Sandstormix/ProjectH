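; Two-sided transition door that teleports the player to a fixed offset from the door behind a camera cutscene.
; Trigger boxes on each side track which side is active and toggle Interact input for the player.
; Interact plays OpeningAnimation and teleports immediately; timelines slide TransitionCamera along Y and swing the door open.
; After a delay, view and control return to the player and the camera moves back.
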(event `self.Side1_TriggerBox.OnComponentBeginOverlap`
  (params (OverlappedComponent :type "PrimitiveComponent Object Reference") (OtherActor :type "Actor Object Reference") (OtherComp :type "PrimitiveComponent Object Reference") (OtherBodyIndex :type Integer) (bFromSweep :type Boolean) (SweepResult :type "HitResult Structure (by ref)"))
  ;[1 1 1] Enable / Disable interact near door
  ;;[1 1 1] Side 1
  (set `self.Side1_active` true)
  (cast `/Game/FirstPerson/Blueprints/BP_FirstPersonCharacter` OtherActor)
  (`self.EnableInput` (`GameplayStatics.GetPlayerController` 0)))

(event `self.Side1_TriggerBox.OnComponentEndOverlap`
  (params (OverlappedComponent :type "PrimitiveComponent Object Reference") (OtherActor :type "Actor Object Reference") (OtherComp :type "PrimitiveComponent Object Reference") (OtherBodyIndex :type Integer))
  ;[1 1 1] Enable / Disable interact near door
  ;;[1 1 1] Side 1
  (set `self.Side1_active` false)
  (cast `/Game/FirstPerson/Blueprints/BP_FirstPersonCharacter` OtherActor)
  (`self.DisableInput` (`GameplayStatics.GetPlayerController` 0)))

(event `self.Side2_TriggerBox.OnComponentBeginOverlap`
  (params (OverlappedComponent :type "PrimitiveComponent Object Reference") (OtherActor :type "Actor Object Reference") (OtherComp :type "PrimitiveComponent Object Reference") (OtherBodyIndex :type Integer) (bFromSweep :type Boolean) (SweepResult :type "HitResult Structure (by ref)"))
  ;[1 1 1] Enable / Disable interact near door
  ;;[1 1 1] Side 2
  (set `self.Side2_active` true)
  (cast `/Game/FirstPerson/Blueprints/BP_FirstPersonCharacter` OtherActor)
  (`self.EnableInput` (`GameplayStatics.GetPlayerController` 0)))

(event `self.Side2_TriggerBox.OnComponentEndOverlap`
  (params (OverlappedComponent :type "PrimitiveComponent Object Reference") (OtherActor :type "Actor Object Reference") (OtherComp :type "PrimitiveComponent Object Reference") (OtherBodyIndex :type Integer))
  ;[1 1 1] Enable / Disable interact near door
  ;;[1 1 1] Side 2
  (set `self.Side2_active` false)
  (cast `/Game/FirstPerson/Blueprints/BP_FirstPersonCharacter` OtherActor)
  (`self.DisableInput` (`GameplayStatics.GetPlayerController` 0)))

(event `InputAction|Interact`
  (params (Key :type "Key Structure"))
  (bind (_returnvalue_x _returnvalue_y _returnvalue_z) (`KismetMathLibrary.BreakVector` (`self.K2_GetActorLocation` self)))
  ;[1 1 1] Door Teleporting
  (:`Pressed`
    (if (`self.Side1_active`)
      (`self.OpeningAnimation`)
      (`self.K2_TeleportTo` :`self` (`GameplayStatics.GetPlayerCharacter` 0) :`DestLocation` (`KismetMathLibrary.MakeVector` (+ _returnvalue_x 50.0) (- _returnvalue_y 100.0) _returnvalue_z)))))

(event `InputAction|Interact`
  (params (Key :type "Key Structure"))
  (bind (_returnvalue_x _returnvalue_y _returnvalue_z) (`KismetMathLibrary.BreakVector` (`self.K2_GetActorLocation` self)))
  ;[1 1 1] Door Teleporting
  (:`Pressed`
    (if (`self.Side2_active`)
      (`self.OpeningAnimation`)
      (`self.K2_TeleportTo` :`self` (`GameplayStatics.GetPlayerCharacter` 0) :`DestLocation` (`KismetMathLibrary.MakeVector` (+ _returnvalue_x 50.0) (+ _returnvalue_y 100.0) _returnvalue_z)))))

(event `OpeningAnimation`
  (bind _returnvalue (`GameplayStatics.GetPlayerController` 0))
  (bind _returnvalue_2 (`GameplayStatics.GetPlayerController` 0))
  (bind _returnvalue_3 (`GameplayStatics.GetPlayerCharacter` 0))
  (bind _transitioncamera (`self.TransitionCamera`))
  (bind (_returnvalue_x _returnvalue_y _returnvalue_z) (`KismetMathLibrary.BreakVector` (`self.K2_GetActorLocation` _transitioncamera)))
  (`self.DisableInput` (`GameplayStatics.GetPlayerCharacter` 0) _returnvalue)
  (`PlayerController.SetViewTargetWithBlend` _returnvalue _transitioncamera 0.0 "VTBlend_Linear" 0.0 false)
  (bind (_direction _dooropen) (`Timeline|CameraPath` :!via `PlayFromStart`)
    (:`Update`
      (`self.K2_SetActorRelativeLocation` _transitioncamera (`KismetMathLibrary.MakeVector` _returnvalue_x (+ _returnvalue_y (`KismetMathLibrary.Lerp` 0.0 2.0 _dooropen)) _returnvalue_z) false false)
      (bind (_direction_2 _dooropen_2) (`Timeline|DoorOpening_Single`)
        (:`Update`
          (`SceneComponent.K2_SetRelativeRotation` (`self.OpeningDoor`) (`KismetMathLibrary.MakeRotator` 0.0 0.0 (`KismetMathLibrary.Lerp` 0.0 80.0 _dooropen_2)) false false)
          (`KismetSystemLibrary.Delay` 4.0)
          (`PlayerController.SetViewTargetWithBlend` _returnvalue_2 _returnvalue_3 0.0 "VTBlend_Linear" 0.0 false)
          (`self.EnableInput` _returnvalue_3 _returnvalue_2)
          (bind (_direction_3 _dooropen_3) (`Timeline|Timeline`)
            (:`Update`
              (`self.K2_SetActorRelativeLocation` _transitioncamera (`KismetMathLibrary.MakeVector` _returnvalue_x (- _returnvalue_y (`KismetMathLibrary.Lerp` 0.0 2.0 _dooropen_3)) _returnvalue_z) false false))))))))

(fn `UserConstructionScript`)